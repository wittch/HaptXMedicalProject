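; Syringe actor that shows liquid changing as its plunger moves while inserted in a medicine bottle, using components named after a screwdriver and bit.
; Overlapping the bottle records the bit's Y position and the liquid's Z scale.
; After three seconds of overlap, Tick sets the liquid's Z scale from bit travel plus the saved amount, hiding it at zero or below.
; Tick resets the delay once overlap ends.
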(event OnComponentBeginOverlap(screwdriver)
  (params (OverlappedComponent :type Primitive%20Component%20Object%20Reference) (OtherActor :type Actor%20Object%20Reference) (OtherComp :type Primitive%20Component%20Object%20Reference) (OtherBodyIndex :type Integer) (bFromSweep :type Boolean) (SweepResult :type Hit%20Result%20Structure%20%28by%20ref%29))
  (bind _asbp_ (Utilities|Casting|CastToBP_ OtherActor))
  (Variables|Default|SetBP_MedicineBottle _asbp_)
  (Variables|Default|SetNewVar_0 true)
  (Variables|Default|SetBitStartLocation (.y (.location (Transformation|GetRelativeTransform (Variables|Default|Getscrewdriver_bit)))))
  (Variables|Default|SetAmount (.z (.scale (Transformation|GetRelativeTransform (Variables|Default|GetLiquid))))))

(event OnComponentEndOverlap(screwdriver)
  (params (OverlappedComponent :type Primitive%20Component%20Object%20Reference) (OtherActor :type Actor%20Object%20Reference) (OtherComp :type Primitive%20Component%20Object%20Reference) (OtherBodyIndex :type Integer))
  (Utilities|Casting|CastToBP_ OtherActor)
  (Variables|Default|SetNewVar_0 false))

(event EventBeginPlay)

(event EventTick
  (params (DeltaSeconds :type Float%20%28single-precision%29))
  (bind _liquid (Variables|Default|GetLiquid))
  (bind _returnvalue (Transformation|GetRelativeTransform _liquid))
  (if (Variables|Default|GetNewVar_0)
    (bind _output_get (Variables|Default|SetElapseTime (- (Variables|Default|GetElapseTime) DeltaSeconds)))
    (if (<= _output_get 0.0)
      (bind _output_get_2 (Variables|Default|SetTotal (- (Math|Float|Absolute(Float) (Variables|Default|GetBitStartLocation)) (.y (.location (Transformation|GetRelativeTransform (Variables|Default|Getscrewdriver_bit)))))))
      (Transformation|SetRelativeTransform (Variables|Default|GetLiquid) (Math|Transform|MakeTransform (.location _returnvalue) (.rotation _returnvalue) (Math|Vector|MakeVector (.x (.scale _returnvalue)) (.y (.scale _returnvalue)) (+ (* _output_get_2 11.0) (Variables|Default|GetAmount)))) false false)
      (if (<= (+ (* _output_get_2 11.0) (Variables|Default|GetAmount)) 0.0)
        (Rendering|SetVisibility (Variables|Default|GetLiquid) false false)
        (else
          (Rendering|SetVisibility (Variables|Default|GetLiquid) true false))))
    (else
      (Variables|Default|SetElapseTime 3.0))))

(fn ConstructionScript)