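; Liquid container actor whose liquid level drops while a syringe (BP_Syringe_COPY) overlaps it.
; BeginPlay caches the Liquid component's initial Z scale, and overlap events on that component store the syringe and toggle an active flag.
; While active, Tick rewrites the liquid's relative transform, setting its Z scale to the initial value minus a fraction of the syringe's Total, clamped at zero.
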(event OnComponentBeginOverlap(Liquid)
  (params (OverlappedComponent :type Primitive%20Component%20Object%20Reference) (OtherActor :type Actor%20Object%20Reference) (OtherComp :type Primitive%20Component%20Object%20Reference) (OtherBodyIndex :type Integer) (bFromSweep :type Boolean) (SweepResult :type Hit%20Result%20Structure%20%28by%20ref%29))
  (bind _asbp_syringe_copy (Utilities|Casting|CastToBP_Syringe_COPY OtherActor))
  (Variables|Default|SetSyringeCopy _asbp_syringe_copy)
  (Variables|Default|SetNewVar_0 true))

(event OnComponentEndOverlap(Liquid)
  (params (OverlappedComponent :type Primitive%20Component%20Object%20Reference) (OtherActor :type Actor%20Object%20Reference) (OtherComp :type Primitive%20Component%20Object%20Reference) (OtherBodyIndex :type Integer))
  (Utilities|Casting|CastToBP_Syringe_COPY OtherActor)
  (Variables|Default|SetNewVar_0 false))

(event EventBeginPlay
  (Variables|Default|SetTotalLiquid (.z (.scale (Transformation|GetRelativeTransform (Variables|Default|GetLiquid))))))

(event EventTick
  (params (DeltaSeconds :type Float%20%28single-precision%29))
  (if (Variables|Default|GetNewVar_0)
    (Utilities|IsValid (Variables|Default|GetLiquid)
      (:Is%20Valid
        (Transformation|SetRelativeTransform (Variables|Default|GetLiquid) (Math|Transform|MakeTransform "0, 0, 0" "0, 0, 0" (Math|Vector|MakeVector 1.0 1.0 (Math|Float|Clamp(Float) (- (Variables|Default|GetTotalLiquid) (* (Variables|/Game/Third/BP_Syringe_COPY.BP_Syringe_COPY_C|GetTotal (Variables|Default|GetSyringeCopy)) 0.1)) 0.0 1e+01))) false false)))))

(fn ConstructionScript)