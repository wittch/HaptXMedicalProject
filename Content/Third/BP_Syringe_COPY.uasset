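; Syringe actor, built on Screwdriver and ScrewdriverBit components, that shows liquid filling while it overlaps a medicine bottle.
; BeginPlay snaps the bit to the Screwdriver's relative location, and overlap events cache the bottle or Human1 and set flags.
; During bottle overlap, Tick converts the 2D distance between both parts into a clamped Liquid Z scale, also stored in NewVar0.
; The Human1 branch on Tick is empty.
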(event OnComponentBeginOverlap(screwdriver)
  (params (OverlappedComponent :type Primitive%20Component%20Object%20Reference) (OtherActor :type Actor%20Object%20Reference) (OtherComp :type Primitive%20Component%20Object%20Reference) (OtherBodyIndex :type Integer) (bFromSweep :type Boolean) (SweepResult :type Hit%20Result%20Structure%20%28by%20ref%29))
  (Utilities|FlowControl|Sequence
    (:then_0
      (bind _asbp_ (Utilities|Casting|CastToBP_ OtherActor))
      (Variables|Default|SetBP_MedicineBottle _asbp_)
      (Variables|Default|SetOverlap?_Syring true))
    (:then_1
      (bind _ashuman_1 (Utilities|Casting|CastToHuman1 OtherActor))
      (Variables|Default|SetHuman1 _ashuman_1)
      (Variables|Default|SetOvelap?_Human1 true))))

(event OnComponentEndOverlap(screwdriver)
  (params (OverlappedComponent :type Primitive%20Component%20Object%20Reference) (OtherActor :type Actor%20Object%20Reference) (OtherComp :type Primitive%20Component%20Object%20Reference) (OtherBodyIndex :type Integer))
  (Utilities|Casting|CastToBP_ OtherActor)
  (Variables|Default|SetOverlap?_Syring false))

(event EventBeginPlay
  (bind _screwdriver (Variables|Default|Getscrewdriver))
  (bind _relativelocation (Variables|/Script/Engine.SceneComponent|GetRelativeLocation _screwdriver))
  (Transformation|SetRelativeLocation (Variables|Default|Getscrewdriver_bit) (Math|Vector|MakeVector (.x _relativelocation) (.y _relativelocation) (.z _relativelocation)) false false))

(event EventTick
  (params (DeltaSeconds :type Float%20%28single-precision%29))
  (bind _liquid (Variables|Default|GetLiquid))
  (bind _screwdriver (Variables|Default|Getscrewdriver))
  (bind _screwdriver_bit (Variables|Default|Getscrewdriver_bit))
  (bind _returnvalue (Transformation|GetRelativeTransform _liquid))
  (bind _returnvalue_2 (Transformation|GetRelativeTransform _screwdriver_bit))
  (bind _returnvalue_3 (Transformation|GetRelativeTransform _screwdriver))
  (Utilities|FlowControl|Sequence
    (:then_0
      (if (Variables|Default|GetOverlap?_Syring)
        (bind _output_get (Variables|Default|SetAmount (Math|Float|Absolute(Float) (Math|Vector|Distance2D(Vector) (Math|Vector2D|MakeVector2D (.x (.location _returnvalue_3)) (.y (.location _returnvalue_3))) (Math|Vector2D|MakeVector2D (.x (.location _returnvalue_2)) (.y (.location _returnvalue_2)))))))
        (Transformation|SetRelativeTransform (Variables|Default|GetLiquid) (Math|Transform|MakeTransform (.location _returnvalue) (.rotation _returnvalue) (Math|Vector|MakeVector 0.5 0.5 (Math|Float|Clamp(Float) (* _output_get 0.1) 0.1 1e+01))) false false)
        (Variables|Default|SetNewVar_0 (Math|Float|Clamp(Float) (* _output_get 0.1) 0.1 1e+01))))
    (:then_1
      (if (Variables|Default|GetOvelap?_Human1)
        _))))

(fn ConstructionScript)