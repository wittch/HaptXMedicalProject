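; Syringe actor whose cylinder stretches with the separation of its two parts while it touches a medicine bottle.
; BeginPlay places ScrewdriverBit at a fixed Y offset from Screwdriver, whose overlap events flag contact with BP_Medicine_Bottle_Duplicate.
; During contact, Tick feeds the hand-computed world distance between both parts into CylinderDuplicate's clamped Z scale, resetting its relative location each frame.
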(event OnComponentBeginOverlap(screwdriver)
  (params (OverlappedComponent :type Primitive%20Component%20Object%20Reference) (OtherActor :type Actor%20Object%20Reference) (OtherComp :type Primitive%20Component%20Object%20Reference) (OtherBodyIndex :type Integer) (bFromSweep :type Boolean) (SweepResult :type Hit%20Result%20Structure%20%28by%20ref%29))
  (Utilities|Casting|CastToBP_Medicine_Bottle_Duplicate OtherActor)
  (Variables|Default|SetIsOverlapped? true))

(event OnComponentEndOverlap(screwdriver)
  (params (OverlappedComponent :type Primitive%20Component%20Object%20Reference) (OtherActor :type Actor%20Object%20Reference) (OtherComp :type Primitive%20Component%20Object%20Reference) (OtherBodyIndex :type Integer))
  (Utilities|Casting|CastToBP_Medicine_Bottle_Duplicate OtherActor)
  (Variables|Default|SetIsOverlapped? false))

(event EventTick
  (params (DeltaSeconds :type Float%20%28single-precision%29))
  (if (Variables|Default|GetIsOverlapped?)
    (bind _output_get (Variables|Default|SetAmount (CallFunction|Distance)))
    (Transformation|SetRelativeTransform (Variables|Default|GetCylinder_Duplicate) (Math|Transform|MakeTransform "0,-5.000000,30.000000" (Variables|/Script/Engine.SceneComponent|GetRelativeRotation (Variables|Default|GetCylinder_Duplicate)) (Math|Vector|MakeVector 0.5 0.5 (Math|Float|Clamp(Float) (* _output_get 0.01) 0.01 1e+01))) false false)))

(event EventBeginPlay
  (bind _screwdriver (Variables|Default|Getscrewdriver))
  (bind _relativelocation (Variables|/Script/Engine.SceneComponent|GetRelativeLocation _screwdriver))
  (Transformation|SetRelativeLocation (Variables|Default|Getscrewdriver_bit) (Math|Vector|MakeVector (.x _relativelocation) (+ (.y _relativelocation) 7e+01) (.z _relativelocation)) false false))

(fn ConstructionScript)

(fn Distance
  (bind _screwdriver (Variables|Default|Getscrewdriver))
  (bind _screwdriver_bit (Variables|Default|Getscrewdriver_bit))
  (bind _returnvalue (Transformation|GetWorldLocation _screwdriver_bit))
  (bind _returnvalue_2 (Transformation|GetWorldLocation _screwdriver))
  (return (Math|Float|Sqrt (+ (Math|Float|Square (- (.x _returnvalue_2) (.x _returnvalue))) (Math|Float|Square (- (.y _returnvalue_2) (.y _returnvalue))) (Math|Float|Square (- (.z _returnvalue_2) (.z _returnvalue)))))))