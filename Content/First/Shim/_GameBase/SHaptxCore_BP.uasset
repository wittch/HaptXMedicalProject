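; SHaptxCore_BP is a HaptX core Blueprint in the game base folder that reports grasp activity as debug text.
; On BeginPlay it calls the parent, then binds handlers to the OnGrasp, OnUpdate and OnRelease dispatchers.
; Each handler only prints a Korean message for grabbed, holding or released, ignoring the supplied component.
; Tick and overlap events are disabled stubs, and the construction script only calls the parent.
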(event Custom|on_grasp
  (params (component :type Primitive%20Component%20Object%20Reference))
  (Development|PrintString "잡음"))

(event Custom|on_release
  (params (component :type Primitive%20Component%20Object%20Reference))
  (Development|PrintString "놓음"))

(event Custom|on_update
  (params (component :type Primitive%20Component%20Object%20Reference))
  (Development|PrintString "잡는중"))

(event EventBeginPlay
  (|CallParentFunction)
  (EventDispatchers|BindEventtoOnGrasp (delegate Custom|on_grasp))
  (EventDispatchers|BindEventtoOnUpdate (delegate Custom|on_update))
  (EventDispatchers|BindEventtoOnRelease (delegate Custom|on_release)))

(event Collision|EventActorBeginOverlap
  (params (OtherActor :type Actor%20Object%20Reference))
  (|CallParentFunction OtherActor) ; 지금 이 노드는 비활성 상태입니다. \n핀을 끌어서 다른 노드를 연결하면 활성화됩니다.
)

(event EventTick
  (params (DeltaSeconds :type Float%20%28single-precision%29))
  (|CallParentFunction DeltaSeconds) ; 지금 이 노드는 비활성 상태입니다. \n핀을 끌어서 다른 노드를 연결하면 활성화됩니다.
)

(fn ConstructionScript
  (|CallParentFunction))