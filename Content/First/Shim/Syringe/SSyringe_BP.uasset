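; Syringe Blueprint with a push component and a cylinder, apparently meant to show the liquid level as the plunger moves.
; BeginPlay caches the push component's starting Y and the cylinder's Z scale.
; Unconnected logic would scale cylinder Z from plunger travel and hide it at zero or below, but it never runs.
; Live behavior beyond that setup is only a debug "Hello" print when SPush overlaps the Box.
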(event OnComponentBeginOverlap(Box)
  (params (OverlappedComponent :type Primitive%20Component%20Object%20Reference) (OtherActor :type Actor%20Object%20Reference) (OtherComp :type Primitive%20Component%20Object%20Reference) (OtherBodyIndex :type Integer) (bFromSweep :type Boolean) (SweepResult :type Hit%20Result%20Structure%20%28by%20ref%29))
  (if (== OtherComp (Variables|Default|GetSPush))
    (Development|PrintString "Hello")))

(event EventBeginPlay
  (Variables|Default|SetCylinderStartPositionY (.y (Variables|/Script/Engine.SceneComponent|GetRelativeLocation (Variables|Default|GetSPush))))
  (Variables|Default|SetLiquid (.z (Variables|/Script/Engine.SceneComponent|GetRelativeScale3D (Variables|Default|GetCylinder)))))

(event EventTick
  (params (DeltaSeconds :type Float%20%28single-precision%29)))

(fn ConstructionScript)